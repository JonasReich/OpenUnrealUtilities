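; Functional test that checks array sorting through the BubbleSortArrayByPredicate node with an A < B predicate.
; On StartTest it sorts the integer array, compares it to the expected result, then sorts the string array, finishing with success or a mismatch error.
; The string check compares the expected array with itself, so it does not validate the sorted strings.
; TestArraySorting is an unimplemented stub.
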(event `self.ReceiveStartTest`
  (bind (_a _b) (`/OpenUnrealUtilities/Runtime/BPML_Object.BubbleSortArrayByPredicate` (`self.TargetArray_Ints`) (< (stale _a) (stale _b)))
    (:`sort finished`
      (if (`KismetArrayLibrary.Array_Identical` (`self.TargetArray_Ints`) (`self.ExpectedSortedResult_Ints`))
        (bind (_a_2 _b_2) (`/OpenUnrealUtilities/Runtime/BPML_Object.BubbleSortArrayByPredicate` (`self.TargetArray_Strings`) (< (stale _a_2) (stale _b_2)))
          (:`sort finished`
            (if (`KismetArrayLibrary.Array_Identical` (`self.ExpectedSortedResult_Strings`) (`self.ExpectedSortedResult_Strings`))
              (`self.FinishTest` "Succeeded")
              (else
                (`self.FinishTest` "Error" "String arrays did not match")))))
        (else
          (`self.FinishTest` "Error" "Int Arrays did not match"))))))

(fn `UserConstructionScript`)