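; Multiplayer test helper actor that signals to the server when a specific client has connected.
; Once its client index is set, the authority waits for that client's player controller (index offset by one) and makes it the actor's owner.
; The remote copy waits until its local controller is the owner, enabling a server RPC that reports a "connected" step, tagged with the client index.
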(event `self.ReceiveBeginPlay`
  (bind _returnvalue (`GameplayStatics.GetPlayerController` (+ (`self.ClientServerIdx`) 1)))
  (`/OpenUnrealUtilities/Runtime/BPML_Actor.WaitUntil` (!= (`self.ClientServerIdx`) -1))
  (`/Engine/EditorBlueprintResources/ActorMacros.Switch Has Authority`
    (:`Authority`
      (`/OpenUnrealUtilities/Runtime/BPML_Actor.WaitUntil` (`KismetSystemLibrary.IsValid` _returnvalue))
      (`self.SetOwner` _returnvalue))
    (:`Remote`
      (`/OpenUnrealUtilities/Runtime/BPML_Actor.WaitUntil` (== (`GameplayStatics.GetPlayerController` 0) (`self.GetOwner`)))
      (`self.SERVER_NotifyClientStep` "connected"))))

(event `SERVER_NotifyClientStep`
  (params (StepName :type Name))
  (`self.ClientStep` StepName (`self.ClientServerIdx`)))

(fn `UserConstructionScript`)